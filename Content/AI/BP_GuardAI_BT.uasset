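; BP_GuardAI_BT is a guard AI Blueprint that handles its own damage and death.
; AnyDamage subtracts damage from Health and plays a sound at the guard's location on either outcome.
; When Health reaches zero or below, it increments KillCount on the player's ThirdPersonCharacter, then destroys itself, using a Sequence so destruction runs even if the cast fails.
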(event Game|Damage|EventAnyDamage
  (params (Damage :type Float%20%28single-precision%29) (DamageType :type Damage%20Type%20Object%20Reference) (InstigatedBy :type Controller%20Object%20Reference) (DamageCauser :type Actor%20Object%20Reference))
  (bind _returnvalue (Transformation|GetActorLocation))
  ;[1 1 1] Health and Death Animation
  (bind _output_get (Variables|Default|SetHealth (- (Variables|Default|GetHealth) Damage)))
  (if (<= _output_get 0.0)
    (Audio|PlaySoundatLocation 0 _returnvalue "0, 0, 0" 1.0 1.0 0.0 0 0 0)
    (Utilities|FlowControl|Sequence
      (:then_0
        ;[1 1 1] Increment number of kills
        (bind _asthird_person_character (Utilities|Casting|CastToThirdPersonCharacter (Game|GetPlayerCharacter 0)))
        (Math|Integer|IncrementInt (Variables|/Game/ThirdPersonBP/Blueprints/ThirdPersonCharacter.ThirdPersonCharacter_C|GetKill%20Count _asthird_person_character)))
      (:then_1
        (Actor|DestroyActor)))
    (else
      (Audio|PlaySoundatLocation 0 _returnvalue "0, 0, 0" 1.0 1.0 0.0 0 0 0))))

(fn ConstructionScript)